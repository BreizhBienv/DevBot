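; BP_JackalSpawner is a labeled spawn point that creates a requested number of Jackal robots.
; SpawnJackals lays out positions in a roughly square grid from the spawner's location, then spawns a BP_JackalRobot at each, possessed by its own instance of the supplied controller class.
; It counts each robot's ready callback and fires OnJackalsReady once all have reported.
; A child billboard text actor displays the spawner's name.
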(event Custom|SpawnJackals
  (params (NumberOfJackals :type Integer) (controller :type Jackal%20Ai%20Controller%20Class%20Reference))
  (Variables|Default|SetCurrentJackalsInitialized 0)
  (bind _output_get (Variables|Default|SetTotalNumberOfJackals NumberOfJackals))
  (bind _spawnpositions (CallFunction|CreateSpawnPositions _output_get))
  (for _array_element _spawnpositions
    (bind _returnvalue (Game|SpawnActorfromClass "/Game/JackalRobot/Pawn/BP_JackalRobot.BP_JackalRobot_C" (Math|Transform|MakeTransform _array_element "0, 0, 0" "1.000000,1.000000,1.000000") "AlwaysSpawn" "MultiplyWithRoot" 0 0))
    (EventDispatchers|BindEventtoJackalReady _returnvalue (delegate Custom|JackalReady_Event))
    (bind _returnvalue_2 (Game|SpawnActorfromClass controller (Math|Transform|MakeTransform "0, 0, 0" "0, 0, 0" "1.000000,1.000000,1.000000") "AlwaysSpawn" "MultiplyWithRoot" 0 0))
    (Pawn|Possess _returnvalue_2 _returnvalue)))

(event Custom|JackalReady_Event
  (bind _result (Math|Integer|IncrementInt (Variables|Default|GetCurrentJackalsInitialized))
    (:%20%20
      (if (>= _result (Variables|Default|GetTotalNumberOfJackals))
        (Default|CallOnJackalsReady)))))

(event EventBeginPlay
  (bind _asbp_billboard_text_render (Utilities|Casting|CastToBP_BillboardTextRender (Variables|/Script/Engine.ChildActorComponent|GetChildActor (Variables|Default|GetBP_BillboardTextRender))))
  (Rendering|Components|TextRender|SetWorldSize (Variables|/Script/Engine.TextRenderActor|GetTextRender _asbp_billboard_text_render) 5e+01)
  (Default|SetText _asbp_billboard_text_render "Jackal 
Spawner"))

(fn ConstructionScript)

(fn CreateSpawnGrid
  (params (NumberOfJackals :type Integer))
  (bind _returnvalue (Math|Conversions|ToFloat(Integer) NumberOfJackals))
  (bind _returnvalue_2 (Math|Float|Sqrt _returnvalue))
  (bind _returnvalue_3 (Math|Float|Ceil _returnvalue_2))
  (if (<= NumberOfJackals 0)
    (return 0 0)
    (else
      (return _returnvalue_3 (/ NumberOfJackals _returnvalue_3)))))

(fn CreateSpawnPositions
  (params (NumberOfJackals :type Integer))
  (bind (_gridx _gridy) (CallFunction|CreateSpawnGrid NumberOfJackals))
  (for _index (range 0 _gridx)
    (for _index_2 (range 0 _gridy)
      (Utilities|Array|Add (LocalVariables|GetFinalSpawnPositions) (+ (Transformation|GetActorLocation) (Math|Vector|MakeVector (* _index 1e+02) (* _index_2 1e+02) 0.0)))
      (bind _result (Math|Integer|IncrementInt (LocalVariables|GetCurrentNbPositions))
        (:%20%20
          (if (>= _result NumberOfJackals)
            (return (LocalVariables|GetFinalSpawnPositions)))))))
  (return (LocalVariables|GetFinalSpawnPositions)))