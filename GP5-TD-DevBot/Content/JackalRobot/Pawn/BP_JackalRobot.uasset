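; Jackal robot pawn, driven by a behavior-tree AI controller, that maps its surroundings, communicates with other robots and travels to stations and targets.
; Sensor scans feed MapMemoryComponent, whose remembered items supply charging station, work station and target choices using controller path queries.
; CommsComponent messages toggle blackboard handshake flags and can pass work-station orders between robots.
; Indicator spheres show power and battery state, while billboards and grid boxes visualize messages and mapping.
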(event OnScanCompleted(Sensor)
  (params (ScanResults :type Array%20of%20Actor%20Object%20References))
  (Class|SpatialMemoryComponent|StoreDetectedActorsArray (Variables|Default|GetMapMemoryComponent) ScanResults))

(event OnMapUpdated(MapMemoryComponent)
  ;[0 0.01475 0.15 0.5] Debug Spatial Grid
  (for _array_element (Variables|/Script/Beryl.SpatialMemoryComponent|GetSpatialGrid (Variables|Default|GetMapMemoryComponent))
    (Utilities|Map|Add (Variables|SpatialGrid|GetSpatialGridDebug) (.CellCoordinates (Utilities|Struct|BreakSpatialGridCell _array_element)) (Math|Color|SelectColor (Math|Color|SelectColor "(R=0.000000,G=1.000000,B=0.000000,A=1.000000)" "(R=0.000000,G=0.000000,B=1.000000,A=1.000000)" (.bIsCellExplored (Utilities|Struct|BreakSpatialGridCell _array_element))) "(R=1.000000,G=0.000000,B=0.000000,A=1.000000)" (.bIsNavigable (Utilities|Struct|BreakSpatialGridCell _array_element))))))

(event Custom|OnPowerChanged_Event
  (params (bIsJackalOn :type Boolean))
  ;[0 0.1838 0.2066 0.5] Battery state display
  (if bIsJackalOn
    (Rendering|Material|SetMaterial (Variables|Default|GetSpherePower) 0 "/Game/JackalRobot/jackal_icons/MI_hmi-indicator_blue.MI_hmi-indicator_blue")
    (Rendering|Material|SetMaterial (Variables|Default|GetSphereComms) 0 "/Game/JackalRobot/jackal_icons/MI_hmi-indicator_green.MI_hmi-indicator_green")
    (CallFunction|SetBatteryIndicator)
    (else
      (Rendering|Material|SetMaterial (Variables|Default|GetSphereWifi) 0 "/Game/JackalRobot/jackal_icons/MI_hmi-indicator_black.MI_hmi-indicator_black"))))

(event Custom|OnBatteryFull_Event
  ;[0 0.1838 0.2066 0.5] Battery state display
  (CallFunction|SetBatteryIndicator))

(event Custom|OnWaitingForMessageIdle
  (params (activate :type Boolean))
  (bind _commscomponent (Variables|Default|GetCommsComponent))
  ;[0 0.1838 0.2066 0.5] Message
  (if activate
    (EventDispatchers|BindEventtoOnMessageReceived _commscomponent (EventDispatchers|CreateEvent :!event CommsREceiverReceiveMessageWhileIdle))
    (else
      (EventDispatchers|UnbindEventfromOnMessageReceived _commscomponent (EventDispatchers|CreateEvent :!event CommsREceiverReceiveMessageWhileIdle)))))

(event Custom|OnWaitingForConnectionEnd
  (params (activate :type Boolean))
  (bind _commscomponent (Variables|Default|GetCommsComponent))
  ;[0 0.1838 0.2066 0.5] Message
  (if activate
    (EventDispatchers|BindEventtoOnMessageReceived _commscomponent (EventDispatchers|CreateEvent :!event CommsReceiverWaitingforConnectionEnd))
    (else
      (EventDispatchers|UnbindEventfromOnMessageReceived _commscomponent (EventDispatchers|CreateEvent :!event CommsReceiverWaitingforConnectionEnd)))))

(event Custom|OnWaitingForResponse
  (params (activate :type Boolean))
  (bind _commscomponent (Variables|Default|GetCommsComponent))
  ;[0 0.1838 0.2066 0.5] Message
  (if activate
    (EventDispatchers|BindEventtoOnMessageReceived _commscomponent (EventDispatchers|CreateEvent :!event CommsSenderReceiveMessageWhileWaitingforAnswer))
    (else
      (EventDispatchers|UnbindEventfromOnMessageReceived _commscomponent (EventDispatchers|CreateEvent :!event CommsSenderReceiveMessageWhileWaitingforAnswer)))))

(event Custom|AddOrderToGoToWorkStation
  ;[0 0.1838 0.2066 0.5] Message
  (EventDispatchers|BindEventtoToExecute (Variables|/Script/Beryl.CommsComponent|GetCurrentMessage (Variables|Default|GetCommsComponent)) (EventDispatchers|CreateEvent :!event OrdertoGotoWorkStation)))

(event Custom|OnBatteryLow_Event
  ;[0 0.1838 0.2066 0.5] Battery state display
  (CallFunction|SetBatteryIndicator))

(event Custom|OnBatteryCritical_Event
  ;[0 0.1838 0.2066 0.5] Battery state display
  (CallFunction|SetBatteryIndicator))

(event Custom|SetBatteryIndicator
  ;[0 0.1838 0.2066 0.5] Battery state display
  (bind _asaic_base_controller (Utilities|Casting|CastToAIC_BaseController (Pawn|GetController))
    (:then
      (Default|OnNewBatteryState _asaic_base_controller (Variables|Default|GetBatteryState)))
    (:CastFailed
      _))
  (switch Utilities|FlowControl|Switch|SwitchonEBatteryState (Variables|Default|GetBatteryState)
    (:BatteryFull
      (Rendering|Material|SetMaterial (Variables|Default|GetSphereBattery) 0 "/Game/JackalRobot/jackal_icons/MI_hmi-indicator_green.MI_hmi-indicator_green" :!label _label))
    (:BatteryHigh
      (goto _label))
    (:BatteryLow
      (Rendering|Material|SetMaterial (Variables|Default|GetSphereBattery) 0 "/Game/JackalRobot/jackal_icons/MI_hmi-indicator_yellow.MI_hmi-indicator_yellow"))
    (:BatteryCritical
      (Rendering|Material|SetMaterial (Variables|Default|GetSphereBattery) 0 "/Game/JackalRobot/jackal_icons/MI_hmi-indicator_red.MI_hmi-indicator_red"))
    (:BatteryEmpty
      (Rendering|Material|SetMaterial (Variables|Default|GetSphereBattery) 0 "/Game/JackalRobot/jackal_icons/MI_hmi-indicator_black.MI_hmi-indicator_black"))))

(event Custom|OnMessageReceived_Event
  (params (Message :type Comms%20Message%20Object%20Reference))
  ;[0 0.1838 0.2066 0.5] Message
  (CallFunction|DisplayMessage Message false))

(event Custom|BroadcastPingMessage
  (bind _self self)
  ;[0 0.1838 0.2066 0.5] Message
  (bind _returnvalue (Class|CommsMessage|CreateCommsMessage _self (Class|JackalRobot|GetJackalId) (Transformation|GetActorLocation _self) _self -1 (Utilities|Time|GetTimeSeconds)))
  (Class|CommsComponent|BroadcastMessage (Variables|Default|GetCommsComponent) _returnvalue))

(event Custom|OnMessageEmitted_Event
  (params (Message :type Comms%20Message%20Object%20Reference))
  ;[0 0.1838 0.2066 0.5] Message
  (CallFunction|DisplayMessage Message true))

(event Custom|DisplayMessage
  (params (Message :type Comms%20Message%20Object%20Reference) (IsEmitter :type Boolean))
  ;[0 0.1838 0.2066 0.5] Message
  (Utilities|IsValid Message
    (:Is%20Valid
      (Utilities|IsValid (Variables|Default|GetCurrentMessageBillboard)
        (:Is%20Valid
          (Components|DestroyComponent (Variables|Default|GetCurrentMessageBillboard)))
        (:Is%20Not%20Valid
          _))
      (bind _returnvalue (AddComponent|AddChildActorComponent false))
      (bind _output_get (Variables|Default|SetCurrentMessageBillboard _returnvalue))
      (bind _asbp_billboard_text_render (Utilities|Casting|CastToBP_BillboardTextRender (Variables|/Script/Engine.ChildActorComponent|GetChildActor _output_get)))
      (Default|SetText _asbp_billboard_text_render (Utilities|String|Append (Utilities|String|SelectString " EMIT:" " RECEIVE:" IsEmitter) " 
Jackal" (Utilities|String|ToString(Integer) (Class|JackalRobot|GetJackalId)) " 
OutID=" (Utilities|String|ToString(Integer) (Variables|/Script/Beryl.CommsMessage|GetSenderID Message)) " 
DestID=" (Utilities|String|ToString(Integer) (Variables|/Script/Beryl.CommsMessage|GetTargetReceiverID Message)) " 
Time=" (Utilities|String|ToString(Text) (Utilities|Text|ToText(Float) (Variables|/Script/Beryl.CommsMessage|GetTimestamp Message) "HalfToEven" false true 1 324 1 1))))
      (Rendering|Components|TextRender|SetWorldSize (Variables|/Script/Engine.TextRenderActor|GetTextRender _asbp_billboard_text_render) 8.0)
      (Transformation|SetWorldLocation (Variables|Default|GetCurrentMessageBillboard) (+ (Transformation|GetWorldLocation (Variables|Default|Getjackal-base)) "0.000000,0.000000,100.000000") false false)
      (Utilities|FlowControl|RetriggerableDelay 7.0)
      (Components|DestroyComponent (Variables|Default|GetCurrentMessageBillboard)))))

(event Custom|OnBatteryHigh_Event
  ;[0 0.1838 0.2066 0.5] Battery state display
  (CallFunction|SetBatteryIndicator))

(event EventTick
  (params (DeltaSeconds :type Float%20%28single-precision%29))
  (Utilities|FlowControl|Sequence
    (:then_0
      (SpatialGrid|DebugSpatialGrid)
      (bind _returnvalue (Class|SpatialMemoryComponent|GetCurrentCellID (Variables|Default|GetMapMemoryComponent)))
      (Rendering|Debug|DrawDebugBox (Class|SpatialMemoryComponent|FromCelltoWorldCoord (Variables|Default|GetMapMemoryComponent) _returnvalue) (/ (Math|Conversions|ToVector(Float) (Class|SpatialMemoryComponent|GetCellSize (Variables|Default|GetMapMemoryComponent))) 2.0) "(R=1.000000,G=0.007447,B=0.978405,A=1.000000)" "0, 0, 0" 0.0 0.0))))

(event EventBeginPlay
  (bind _commscomponent (Variables|Default|GetCommsComponent))
  ;[0 0.2865 0.1311 0.722] BeginPlay
  (Variables|Default|SetBodyMesh (Variables|Default|Getjackal-base))
  (Variables|Default|SetWheelRearRight (Variables|Default|Getjackal-wheel_rear_right))
  (Variables|Default|SetWheelRearLeft (Variables|Default|Getjackal-wheel-rear_left))
  (Variables|Default|SetWheelFrontLeft (Variables|Default|Getjackal-wheel-front_left))
  (Variables|Default|SetWheelFrontRight (Variables|Default|Getjackal-wheel-front_right))
  (Variables|/Script/Beryl.CommsComponent|SetCommsArea _commscomponent (Variables|Default|GetCommsCollision))
  (EventDispatchers|BindEventtoOnMessageEmitted _commscomponent (EventDispatchers|CreateEvent :!event Custom|OnMessageEmitted_Event))
  (EventDispatchers|AssignOnMessageReceived _commscomponent (EventDispatchers|CreateEvent :!event Custom|OnMessageReceived_Event))
  (CallFunction|OnWaitingforMessageIdle true)
  (EventDispatchers|AssignOnPowerChanged (delegate Custom|OnPowerChanged_Event))
  (EventDispatchers|AssignOnBatteryFull (delegate Custom|OnBatteryFull_Event))
  (EventDispatchers|BindEventtoOnBatteryHigh (delegate Custom|OnBatteryHigh_Event))
  (EventDispatchers|AssignOnBatteryLow (delegate Custom|OnBatteryLow_Event))
  (EventDispatchers|AssignOnBatteryCritical (delegate Custom|OnBatteryCritical_Event))
  (Utilities|FlowControl|DelayUntilNextTick)
  (SpatialGrid|AddFirstCell)
  (Default|CallJackalReady))

(fn ConstructionScript)

(fn RetrieveClosestChargingStation
  (bind _asaic_base_controller (Utilities|Casting|CastToAIC_BaseController (Pawn|GetController))
    (:then
      (bind (_keypin _valuepin) (Utilities|Map|ForEachLoop(Map) (Class|SpatialMemoryComponent|GetSpatialItemsMemory (Variables|Default|GetMapMemoryComponent)))
        (:then
          (if (Utilities|Enum|Equal(Enum) (.DetectedObject (Utilities|Struct|BreakSpatialMemoryElement _valuepin)) "ChargingStation")
            (bind (_returnvalue _path_points) (Default|GetPath _asaic_base_controller (.Location (Utilities|Struct|BreakSpatialMemoryElement _valuepin))))
            (if (or (< (LocalVariables|GetBestCharginStation) 0) (< _returnvalue (LocalVariables|GetBestLength)))
              (LocalVariables|SetBestPath _path_points)
              (LocalVariables|SetBestLength _returnvalue)
              (LocalVariables|SetBestCharginStation _keypin))))
        (:CompletedPin
          (return (LocalVariables|GetBestCharginStation) (LocalVariables|GetBestPath)))))
    (:CastFailed
      (Development|PrintString "CouldNotFindAiController")
      (return -1 0))))

(fn AddFirstCell
  (bind _mapmemorycomponent (Variables|Default|GetMapMemoryComponent))
  (bind _returnvalue (Class|SpatialMemoryComponent|GetCurrentCellID _mapmemorycomponent))
  (Class|SpatialMemoryComponent|AddCell _mapmemorycomponent _returnvalue))

(fn DebugSpatialGrid
  (if (Variables|SpatialGrid|GetbDebugSpatialGrid)
    (bind (_keypin _valuepin) (Utilities|Map|ForEachLoop(Map) (Variables|SpatialGrid|GetSpatialGridDebug))
      (:then
        (Rendering|Debug|DrawDebugBox (Class|SpatialMemoryComponent|FromCelltoWorldCoord (Variables|Default|GetMapMemoryComponent) _keypin) (/ (- (Math|Conversions|ToVector(Float) (Class|SpatialMemoryComponent|GetCellSize (Variables|Default|GetMapMemoryComponent))) "10.000000,10.000000,10.000000") 2.0) _valuepin "0, 0, 0" 0.0 0.0)))))

(fn IsSpeedClosetoZero
  (return (Math|Float|NearlyEqual(Float) (Variables|Default|GetLinearSpeed) 0.0 0.1)))

(fn ForwardLineTrace
  (bind _sensor (Variables|Default|GetSensor))
  (bind _returnvalue (Transformation|GetWorldLocation _sensor))
  (bind _outhit (Collision|LineTraceByChannel _returnvalue (+ _returnvalue (* (Math|Vector|RotateVectorAroundAxis (Math|Vector|GetForwardVector (Variables|Default|GetBodyMesh)) -1e+01 (Math|Vector|GetRightVector (Variables|Default|GetBodyMesh))) (Variables|Default|GetForwardLineTraceDistance))) "TraceTypeQuery3" false 0 "ForDuration" true "(R=1.000000,G=0.000000,B=0.000000,A=1.000000)" "(R=0.000000,G=1.000000,B=0.000000,A=1.000000)" 2.0))
  (return _outhit))

(fn CommsSenderReceiveMessageWhileWaitingforAnswer
  (params (Message :type Comms%20Message%20Object%20Reference))
  (if (not (Utilities|Array|ContainsItem (Variables|/Script/Beryl.CommsComponent|GetCommsTarget (Variables|Default|GetCommsComponent)) (Variables|/Script/Beryl.JackalRobot|GetCommsComponent (Variables|/Script/Beryl.CommsMessage|GetSenderComponent Message))))
    (Utilities|Array|AddUnique (Variables|/Script/Beryl.CommsComponent|GetCommsTarget (Variables|Default|GetCommsComponent)) (Variables|/Script/Beryl.JackalRobot|GetCommsComponent (Variables|/Script/Beryl.CommsMessage|GetSenderComponent Message)))
    (AI|Components|Blackboard|SetValueasBool (AI|GetBlackboard 0) (Utilities|Name|MakeLiteralName "IsConnectionEstablished") true)
    (else
      (bind _returnvalue (Utilities|Array|RemoveItem (Variables|/Script/Beryl.CommsComponent|GetCommsTarget (Variables|Default|GetCommsComponent)) (Variables|/Script/Beryl.JackalRobot|GetCommsComponent (Variables|/Script/Beryl.CommsMessage|GetSenderComponent Message)))))))

(fn CommsReceiverReceiveMessageWhileIdle
  (params (Message :type Comms%20Message%20Object%20Reference))
  (AI|Components|Blackboard|SetValueasBool (AI|GetBlackboard 0) (Utilities|Name|MakeLiteralName "HasReceivedPing") true)
  (Utilities|Array|AddUnique (Variables|/Script/Beryl.CommsComponent|GetCommsTarget (Variables|Default|GetCommsComponent)) (Variables|/Script/Beryl.JackalRobot|GetCommsComponent (Variables|/Script/Beryl.CommsMessage|GetSenderComponent Message))))

(fn CommsReceiverWaitingforConnectionEnd
  (params (Message :type Comms%20Message%20Object%20Reference))
  (bind _self self)
  (Comms|CleanCommunicationData)
  (bind _returnvalue (Class|CommsMessage|CreateCommsMessage _self (Class|JackalRobot|GetJackalId) (Transformation|GetActorLocation self) _self -1 (Utilities|Time|GetTimeSeconds)))
  (Class|CommsComponent|SendMessagetoTarget (Variables|Default|GetCommsComponent) (Variables|/Script/Beryl.JackalRobot|GetCommsComponent (Variables|/Script/Beryl.CommsMessage|GetSenderComponent Message)) _returnvalue))

(fn CleanCommunicationData
  (bind _returnvalue (AI|GetBlackboard 0))
  (bind _commscomponent (Variables|Default|GetCommsComponent))
  (Variables|/Script/Beryl.CommsComponent|SetLastPingTimeStamp (Variables|Default|GetCommsComponent) (Utilities|Time|GetGameTimeinSeconds))
  (AI|Components|Blackboard|SetValueasBool _returnvalue (Utilities|Name|MakeLiteralName "IsCommunicating") false)
  (AI|Components|Blackboard|SetValueasBool _returnvalue (Utilities|Name|MakeLiteralName "IsWaitingForResponse") false)
  (AI|Components|Blackboard|SetValueasBool _returnvalue (Utilities|Name|MakeLiteralName "HasReceivedPing") false)
  (AI|Components|Blackboard|SetValueasBool _returnvalue (Utilities|Name|MakeLiteralName "IsConnectionEstablished") false)
  (AI|Components|Blackboard|SetValueasBool _returnvalue (Utilities|Name|MakeLiteralName "IsInitiator") false)
  (Utilities|Array|Clear (Variables|/Script/Beryl.CommsComponent|GetCommsTarget _commscomponent))
  (Variables|/Script/Beryl.CommsComponent|SetCurrentMessage _commscomponent 0)
  (CallFunction|OnWaitingforMessageIdle true)
  (CallFunction|OnWaitingforResponse false)
  (CallFunction|OnWaitingforConnectionEnd false))

(fn RetrieveTaskwithReward
  (params (TaskType :type EInteractivePropType%20Enum :default "Unknown"))
  (bind (_keypin _valuepin) (Utilities|Map|ForEachLoop(Map) (Class|SpatialMemoryComponent|GetSpatialItemsMemory (Variables|Default|GetMapMemoryComponent)))
    (:then
      (if (and (Utilities|Enum|Equal(Enum) (.DetectedObject (Utilities|Struct|BreakSpatialMemoryElement _valuepin)) TaskType) (> (.ElementReward (Utilities|Struct|BreakSpatialMemoryElement _valuepin)) 0.0))
        (Utilities|Array|AddUnique (LocalVariables|GetToVisit) _keypin)))
    (:CompletedPin
      (return (LocalVariables|GetToVisit)))))

(fn AnyNonVisitedDedicatedTarget
  (bind _tovisit (Task|RetrieveTaskwithReward "JackalTarget"))
  (for _array_element _tovisit
    (if (== (Utilities|Array|FindItem (Variables|Task|GetDedicatedTargetVisited) _array_element) -1)
      (Utilities|Array|AddUnique (LocalVariables|GetVisitable) _array_element)))
  (return (LocalVariables|GetVisitable)))

(fn GetClosestSpatialTarget
  (params (InItems :type Array%20of%20Integers))
  (bind _asaic_jackal_btcontroller (Utilities|Casting|CastToAIC_JackalBTController (AI|GetAIController self)))
  (LocalVariables|SetBtController _asaic_jackal_btcontroller)
  (for _array_element InItems
    (bind (_returnvalue _path_points) (Default|GetPath (LocalVariables|GetBtController) (.Location (Utilities|Struct|BreakSpatialMemoryElement (.Value (Utilities|Map|Find (Class|SpatialMemoryComponent|GetSpatialItemsMemory (Variables|Default|GetMapMemoryComponent)) _array_element))))))
    (if (or (< (LocalVariables|GetBestTarget) 0) (> _returnvalue (LocalVariables|GetBestDist)))
      (LocalVariables|SetBestDist _returnvalue)
      (LocalVariables|SetBestTarget _array_element)
      (LocalVariables|SetBestPathPoints _path_points)))
  (return (LocalVariables|GetBestTarget) (LocalVariables|GetBestPathPoints)))

(fn SetNewPath
  (params (NewTarget :type Integer) (NewPath :type Array%20of%20Vectors))
  (bind _asaic_jackal_btcontroller (Utilities|Casting|CastToAIC_JackalBTController (AI|GetAIController self)))
  (Default|SetNewPath _asaic_jackal_btcontroller NewPath)
  (Variables|Default|SetCurrentTarget NewTarget))

(fn StopJackal
  (bind _asaic_jackal_btcontroller (Utilities|Casting|CastToAIC_JackalBTController (AI|GetAIController self)))
  (Default|StopJackal _asaic_jackal_btcontroller)
  (Variables|Default|SetCurrentTarget -1))

(fn RetrieveChargingStations
  (bind (_keypin _valuepin) (Utilities|Map|ForEachLoop(Map) (Class|SpatialMemoryComponent|GetSpatialItemsMemory (Variables|Default|GetMapMemoryComponent)))
    (:then
      (if (Utilities|Enum|Equal(Enum) (.DetectedObject (Utilities|Struct|BreakSpatialMemoryElement _valuepin)) "ChargingStation")
        (Utilities|Array|AddUnique (LocalVariables|GetToVisit) _keypin)))
    (:CompletedPin
      (return (LocalVariables|GetToVisit)))))

(fn RetrieveWorkingStation
  (Utilities|FlowControl|Sequence
    (:then_0
      (bind (_keypin _valuepin) (Utilities|Map|ForEachLoop(Map) (Class|SpatialMemoryComponent|GetSpatialItemsMemory (Variables|Default|GetMapMemoryComponent)))
        (:then
          (if (Utilities|Enum|Equal(Enum) (.DetectedObject (Utilities|Struct|BreakSpatialMemoryElement _valuepin)) "WorkStation")
            (Utilities|Array|AddUnique (LocalVariables|GetWorkStations) _keypin)))))
    (:then_1
      (Class|KismetArrayLibrary|SortIntArray (LocalVariables|GetWorkStations))
      (LocalVariables|SetItemIndex (Utilities|Array|FindItem (LocalVariables|GetWorkStations) (Variables|Task|GetCurrentWorkStation)))
      (if (== (LocalVariables|GetItemIndex) -1)
        (bind _tovisit (Task|RetrieveTaskwithReward "WorkStation"))
        (bind (_targettovisit _pathtotake) (Task|GetClosestSpatialTarget _tovisit))
        (return _targettovisit _pathtotake)
        (else
          (bind (_outputpin _path_points) (|RetrieveNextStationWithReward))
          (return _outputpin _path_points))))))

(fn OrdertoGotoWorkStation
  (params (Sender :type Jackal%20Robot%20Object%20Reference) (Other :type Jackal%20Robot%20Object%20Reference))
  (bind _asbp_jackal_robot (Utilities|Casting|CastToBP_JackalRobot Sender))
  (bind _asbp_jackal_robot_2 (Utilities|Casting|CastToBP_JackalRobot Other))
  (LocalVariables|SetCastedOther _asbp_jackal_robot_2)
  (bind _output_get (Variables|BP_JackalRobot_C|SetCurrentWorkStation (LocalVariables|GetCastedOther) (Variables|BP_JackalRobot_C|GetCurrentWorkStation _asbp_jackal_robot)))
  (bind _asaic_jackal_btcontroller (Utilities|Casting|CastToAIC_JackalBTController (AI|GetAIController (LocalVariables|GetCastedOther))))
  (bind _path_points (Default|GetPath _asaic_jackal_btcontroller (.Location (Utilities|Struct|BreakSpatialMemoryElement (.Value (Utilities|Map|Find (Class|SpatialMemoryComponent|GetSpatialItemsMemory (Variables|/Script/Beryl.JackalRobot|GetMapMemoryComponent (LocalVariables|GetCastedOther))) _output_get))))))
  (CallFunction|SetNewPath (LocalVariables|GetCastedOther) _output_get _path_points))