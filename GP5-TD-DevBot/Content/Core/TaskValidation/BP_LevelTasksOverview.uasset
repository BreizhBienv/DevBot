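; Level task tracker that scores Jackal robots on rewarded props against an optional time limit, shown on a billboard.
; It binds to each prop's task-finished event and ends the level when all tasks complete or time expires.
; In test mode it benchmarks AI architectures, respawning Jackals with the selected controller class.
; Each run is stored in the GameInstance and the level reloads, preserving player transform, until the last run exports CSV.
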(event Custom|InitAllTasks
  ;[0 0.1838 0.2066 0.5] Begin Play
  (Variables|Default|SetNumberOfTasks 0)
  (Variables|Default|SetCurrentCompletedTasks 0)
  (Variables|Default|SetTotalReward 0.0)
  (Variables|Default|SetCurrentReward 0.0)
  (bind _outactors (Actor|GetAllActorsOfClass "/Script/Beryl.JackalInteractiveProp"))
  (for _array_element _outactors
    (if (> (Variables|/Script/Beryl.JackalInteractiveProp|GetReward _array_element) 0.0)
      (EventDispatchers|BindEventtoOnTaskFinished _array_element (delegate Custom|OnTaskFinished))
      (Math|Integer|IncrementInt (Variables|Default|GetNumberOfTasks)
        (:%20%20
          (Variables|Default|SetTotalReward (+ (Variables|Default|GetTotalReward) (Variables|/Script/Beryl.JackalInteractiveProp|GetReward _array_element)))))))
  (bind _outactors_2 (Actor|GetAllActorsOfClass "/Game/JackalInteractiveProps/BP_DedicatedJackalTarget.BP_DedicatedJackalTarget_C"))
  (for _array_element_2 _outactors_2
    (Default|AssigntoRandomJackal _array_element_2)
    (CallFunction|UpdateText)))

(event Custom|OnTaskFinished
  (params (RewardObtained :type Float%20%28single-precision%29))
  ;[0 0.1838 0.2066 0.5] Update
  (if (not (Variables|Default|GetLevelComplete))
    (Variables|Default|SetCurrentReward (+ RewardObtained (Variables|Default|GetCurrentReward)))
    (Math|Integer|IncrementInt (Variables|Default|GetCurrentCompletedTasks)
      (:%20%20
        (if (== (Variables|Default|GetCurrentCompletedTasks) (Variables|Default|GetNumberOfTasks))
          (CallFunction|CompleteLevel true))
        (CallFunction|Updatetext)))))

(event Custom|InitLevel
  ;[0 0.1838 0.2066 0.5] Begin Play
  (bind _asgi_test_save_data (Utilities|Casting|CastToGI_TestSaveData (Game|GetGameInstance)))
  (Variables|Default|SetCurrentTest (Variables|/Game/Core/TaskValidation/GI_TestSaveData.GI_TestSaveData_C|GetCurrentTest _asgi_test_save_data))
  (Variables|Default|SetLevelComplete false)
  (if (> (.x (.Scale (Math|Transform|BreakTransform (Variables|/Game/Core/TaskValidation/GI_TestSaveData.GI_TestSaveData_C|GetPreviousPlayerPawnTransform _asgi_test_save_data)))) 0.1)
    (Transformation|SetActorTransform (Game|Player|GetPlayerPawn 0) (Variables|/Game/Core/TaskValidation/GI_TestSaveData.GI_TestSaveData_C|GetPreviousPlayerPawnTransform _asgi_test_save_data)))
  (CallFunction|StartLevelTimer)
  (if (Variables|Default|GetIsInTestMode)
    (CallFunction|InitJackals)
    (else
      (CallFunction|InitAllTasks))))

(event Custom|OnJackalsReady_Event
  ;[0 0.1838 0.2066 0.5] Begin Play
  (Utilities|FlowControl|DelayUntilNextTick)
  (CallFunction|InitAllTasks))

(event Custom|UpdateText
  ;[0 0.1838 0.2066 0.5] Update
  (Default|SetText (Variables|Default|GetBillboardText) (Utilities|String|Append (Utilities|String|Append (Utilities|String|SelectString "-FINISHED- 
" "-IN PROGRESS- 
" (Variables|Default|GetLevelComplete)) "Level Tasks: 
" (Utilities|String|SelectString (Utilities|String|Append "Time:  " (Utilities|String|ToString(Text) (Utilities|Text|ToText(Float) (Variables|Default|GetLevelRemainingTime) "HalfToEven" false true 3 324 1 1)) "/" (Utilities|String|ToString(Text) (Utilities|Text|ToText(Float) (Variables|Default|GetMaxLevelTime) "HalfToEven" false true 3 324 1 1)) " 
") "" (>= (Variables|Default|GetMaxLevelTime) 0.0)) "Completed: ") (Utilities|String|ToString(Integer) (Variables|Default|GetCurrentCompletedTasks)) "/" (Utilities|String|ToString(Integer) (Variables|Default|GetNumberOfTasks)) " 
Reward: " (Utilities|String|ToString(Text) (Utilities|Text|ToText(Float) (Variables|Default|GetCurrentReward) "HalfToEven" false true 1 324 0 1)) "/" (Utilities|String|ToString(Text) (Utilities|Text|ToText(Float) (Variables|Default|GetTotalReward) "HalfToEven" false true 1 324 0 1)) (Utilities|String|SelectString (Utilities|String|Append " 
Test " (Utilities|String|ToString(Integer) (+ (Variables|Default|GetCurrentTest) 1)) "/" (Utilities|String|ToString(Integer) (Variables|Default|GetNumberOfTests))) "" (Variables|Default|GetIsInTestMode)) " 
------")))

(event Custom|InitBillboard
  ;[0 0.1838 0.2066 0.5] Begin Play
  (bind _asbp_billboard_text_render (Utilities|Casting|CastToBP_BillboardTextRender (Variables|/Script/Engine.ChildActorComponent|GetChildActor (Variables|Default|GetBP_BillboardTextRender))))
  (bind _output_get (Variables|Default|SetBillboardText _asbp_billboard_text_render))
  (Rendering|Components|TextRender|SetWorldSize (Variables|/Script/Engine.TextRenderActor|GetTextRender _output_get) 1e+02)
  (Default|SetVerticallyCentered _output_get true))

(event Custom|CompleteLevel
  (params (success :type Boolean))
  ;[0 0.1838 0.2066 0.5] Level Complete
  (Variables|Default|SetLevelComplete true)
  (Variables|Default|SetLevelRemainingTime 0.0)
  (CallFunction|UpdateText)
  (Actor|Tick|SetActorTickEnabled false)
  (if (Variables|Default|GetIsInTestMode)
    (CallFunction|SaveTestData)
    (elif (Variables|Default|GetTurnOffJackalsOnEnd)
      (bind _outactors (Actor|GetAllActorsOfClass "/Script/Beryl.JackalRobot"))
      (for _array_element _outactors
        (Class|JackalRobot|SetJackalPower _array_element false)))))

(event Custom|SaveTestData
  ;[0 0.1838 0.2066 0.5] Level Complete
  ;;[1 0.7288 0 1 30] A COMPLETER: Ajouter des données si jugé nécessaire
  (bind _asgi_test_save_data (Utilities|Casting|CastToGI_TestSaveData (Game|GetGameInstance)))
  (bind _returnvalue (Game|GetCurrentLevelName true))
  (bind _outactors (Actor|GetAllActorsOfClass 0))
  (Default|AddNewTestData _asgi_test_save_data (Utilities|Array|Length _outactors) (Variables|Default|GetCurrentReward) (Variables|Default|GetTotalReward) (- (Variables|Default|GetMaxLevelTime) (Variables|Default|GetLevelRemainingTime)) (Utilities|String|EnumtoString (Variables|Default|GetBotTypeTested)) _returnvalue (Variables|Default|GetMaxLevelTime))
  (if (>= (Variables|Default|GetCurrentTest) (- (Variables|Default|GetNumberOfTests) 1))
    (Class|CSVDataSaverComponent|SaveStringasCSV (Variables|Default|GetCSVDataSaver) (.Header (Default|GetSaveDataasString _asgi_test_save_data)) (.StrData (Default|GetSaveDataasString _asgi_test_save_data)))
    (else
      (CallFunction|RestartTest))))

(event Custom|RestartTest
  ;[0 0.1838 0.2066 0.5] Level Complete
  ;;[1 0.7288 0 1 30] A COMPLETER: Ajouter des données si jugé nécessaire
  (bind _asgi_test_save_data (Utilities|Casting|CastToGI_TestSaveData (Game|GetGameInstance))
    (:then
      (Variables|/Game/Core/TaskValidation/GI_TestSaveData.GI_TestSaveData_C|SetPreviousPlayerPawnTransform _asgi_test_save_data (Transformation|GetActorTransform (Game|Player|GetPlayerPawn 0))))
    (:CastFailed
      _))
  (bind _returnvalue (Game|GetCurrentLevelName true))
  (Game|OpenLevel(byName) (Utilities|String|StringToName _returnvalue)))

(event Custom|StartLevelTimer
  ;[0 0.1838 0.2066 0.5] Begin Play
  (if (> (Variables|Default|GetMaxLevelTime) 0.0)
    (Actor|Tick|SetActorTickEnabled true)
    (Variables|Default|SetLevelRemainingTime (Variables|Default|GetMaxLevelTime))
    (else
      (Actor|Tick|SetActorTickEnabled false))))

(event Custom|InitJackals
  ;[0 0.1838 0.2066 0.5] Begin Play
  (bind _outactors (Actor|GetAllActorsOfClass "/Game/JackalRobot/Pawn/BP_JackalRobot.BP_JackalRobot_C"))
  (for _array_element _outactors
    (Actor|DestroyActor _array_element))
  (Utilities|FlowControl|DelayUntilNextTick)
  (bind _jackalspawner (Variables|Default|GetJackalSpawner)
    (:then
      (Default|SpawnJackals _jackalspawner (Variables|Default|GetNumberOfJackals) (CallFunction|ControllerEnumtoClass (Variables|Default|GetBotTypeTested))))
    (:else)))

(event EventBeginPlay
  ;[0 0.1838 0.2066 0.5] Begin Play
  (CallFunction|InitBillboard)
  (bind _returnvalue (Actor|GetActorOfClass "/Game/JackalRobot/BP_JackalSpawner.BP_JackalSpawner_C"))
  (bind _output_get (Variables|Default|SetJackalSpawner _returnvalue))
  (Utilities|IsValid _output_get
    (:Is%20Valid
      (EventDispatchers|BindEventtoOnJackalsReady (Variables|Default|GetJackalSpawner) (delegate Custom|OnJackalsReady_Event)))
    (:Is%20Not%20Valid
      _))
  (CallFunction|InitLevel))

(event EventTick
  (params (DeltaSeconds :type Float%20%28single-precision%29))
  ;[0 0.1838 0.2066 0.5] Update
  (if (not (Variables|Default|GetLevelComplete))
    (Variables|Default|SetLevelRemainingTime (- (Variables|Default|GetLevelRemainingTime) DeltaSeconds))
    (if (<= (Variables|Default|GetLevelRemainingTime) 0.0)
      (CallFunction|CompleteLevel false)
      (else
        (CallFunction|UpdateText)))))

(fn ConstructionScript)

(fn TestDatatoCSVString)

(fn SaveCurrentTest
  (bind _asgi_test_save_data (Utilities|Casting|CastToGI_TestSaveData (Game|GetGameInstance))
    (:then
      (bind _outactors (Actor|GetAllActorsOfClass "/Game/JackalRobot/Pawn/BP_JackalRobot.BP_JackalRobot_C"))
      (Default|AddNewTestData _asgi_test_save_data (Utilities|Array|Length _outactors) (Variables|Default|GetCurrentReward) (Variables|Default|GetTotalReward) 0.0 "" "" 0.0))
    (:CastFailed
      (return false))))

(fn ControllerEnumtoClass
  (params (ControllerEnum :type E_BotTypes%20Enum :default "NewEnumerator0"))
  (switch Utilities|FlowControl|Switch|SwitchonE_BotTypes ControllerEnum
    (:NewEnumerator0
      (return "/Game/Bots/BT/AIC_JackalBTController.AIC_JackalBTController_C"))
    (:NewEnumerator1
      (return "/Game/Bots/UtilityAI/AIC_JackalUtilityAIController.AIC_JackalUtilityAIController_C"))
    (:NewEnumerator2
      (return "/Game/Bots/GOAP/AIC_JackalGOAPController.AIC_JackalGOAPController_C"))
    (:NewEnumerator3
      (return "/Game/Bots/FSM/AIC_JackalFSMController.AIC_JackalFSMController_C"))
    (:NewEnumerator4
      (return "/Game/Bots/AiController/AIC_TestController.AIC_TestController_C"))))