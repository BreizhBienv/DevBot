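; BP_BillboardTextRender is a debug text actor that keeps its TextRender facing the player camera.
; BeginPlay caches the camera component of player pawn 0, and every Tick rotates the text with a look-at rotation toward it while that camera is valid.
; Events let callers set the displayed text and switch vertical alignment between centered and top.
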(event Custom|UpdateTextRotation
  (bind _playercamera (Variables|Default|GetPlayerCamera)
    (:then
      (Transformation|SetWorldRotation (Variables|Default|GetTextRender) (Math|Rotator|FindLookatRotation (Transformation|GetWorldLocation (Variables|Default|GetTextRender)) (Transformation|GetWorldLocation _playercamera)) false false))
    (:else)))

(event Custom|SetText
  (params (NewText :type String))
  (Rendering|Components|TextRender|SetText (Variables|Default|GetTextRender) (Utilities|Text|ToText(String) NewText)))

(event Custom|SetVerticallyCentered
  (params (newVerticallyCentered :type Boolean))
  (bind _textrender (Variables|Default|GetTextRender))
  (if newVerticallyCentered
    (Class|TextRenderComponent|SetVerticalAlignment _textrender "EVRTA_TextCenter")
    (else
      (Class|TextRenderComponent|SetVerticalAlignment _textrender "EVRTA_TextTop"))))

(event EventBeginPlay
  (Variables|Default|SetPlayerCamera (Actor|GetComponentbyClass (Game|Player|GetPlayerPawn 0) "/Script/Engine.CameraComponent")))

(event EventTick
  (params (DeltaSeconds :type Float%20%28single-precision%29))
  (CallFunction|UpdateTextRotation))

(fn ConstructionScript)