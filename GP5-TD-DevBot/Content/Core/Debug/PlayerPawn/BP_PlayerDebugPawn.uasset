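; Debug player pawn that flies a free camera and lets the player inspect and select Jackal robots.
; On BeginPlay it sets fullscreen mode, adds the debug input mapping and creates the Jackal debug UI widget.
; A per-tick cursor trace feeds the hovered robot to the UI, and left click makes it the current one.
; Enhanced Input drives camera-relative movement, mouse axes look, Ctrl toggles the cursor and Escape quits.
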(event Custom|UpdateHoveredJackal
  (params (jackal :type BP%20Jackal%20Robot%20Object%20Reference))
  (bind _jackalcontrolui (Variables|Default|GetjackalControlUI))
  ;[0 0.7604 0.5839] Select robot
  (bind _output_get (Variables|Default|SethoveredJackal jackal))
  (Utilities|IsValid _output_get
    (:Is%20Valid
      (Default|UpdateHoveredJackal _jackalcontrolui _output_get))
    (:Is%20Not%20Valid
      (Default|UpdateHoveredJackal _jackalcontrolui))))

(event Input|EnhancedActionEvents|EnhancedInputActionIA_MoveForward
  (params (ActionValue :type Float%20%28double-precision%29) (ElapsedSeconds :type Float%20%28double-precision%29) (TriggeredSeconds :type Float%20%28double-precision%29) (InputAction :type Input%20Action%20Object%20Reference :default "/Game/Core/Debug/PlayerPawn/IA_MoveForward.IA_MoveForward"))
  ;[0 0.7604 0.5839] Movement
  (Class|PawnMovementComponent|AddInputVector (Variables|Default|GetFloatingPawnMovement) (* (Math|Vector|GetForwardVector (Transformation|GetWorldRotation (Variables|Default|GetCamera))) ActionValue (Math|Float|MakeLiteralFloat 0.8) (Variables|Default|Getspeed)) true))

(event Input|EnhancedActionEvents|EnhancedInputActionIA_MoveLeft
  (params (ActionValue :type Float%20%28double-precision%29) (ElapsedSeconds :type Float%20%28double-precision%29) (TriggeredSeconds :type Float%20%28double-precision%29) (InputAction :type Input%20Action%20Object%20Reference :default "/Game/Core/Debug/PlayerPawn/IA_MoveLeft.IA_MoveLeft"))
  ;[0 0.7604 0.5839] Movement
  (Class|PawnMovementComponent|AddInputVector (Variables|Default|GetFloatingPawnMovement) (* (Math|Vector|GetRightVector (Transformation|GetWorldRotation (Variables|Default|GetCamera))) ActionValue (Math|Float|MakeLiteralFloat 0.8) (Variables|Default|Getspeed)) true))

(event EventBeginPlay
  ;[0 0.7604 0.5839] BeginPlay
  (bind _returnvalue (Settings|GetGameUserSettings))
  (Class|GameUserSettings|SetFullscreenMode _returnvalue "Fullscreen")
  (bind _output_get (Variables|Default|SetlocalController (Game|GetPlayerController 0)))
  (Input|AddMappingContext (PlayerController|LocalPlayerSubsystems|GetEnhancedInputLocalPlayerSubsystem _output_get) "/Game/Core/Debug/PlayerPawn/IMC_DebugPawnInputs.IMC_DebugPawnInputs" 1 (Utilities|Struct|MakeModifyContextOptions true true false))
  (Input|EnableInput (Variables|Default|GetlocalController))
  (bind _returnvalue_2 (UserInterface|CreateWidget "/Game/Core/Debug/PlayerPawn/WBP_JackalDebugUI.WBP_JackalDebugUI_C" (Variables|Default|GetlocalController)))
  (bind _output_get_2 (Variables|Default|SetjackalControlUI _returnvalue_2))
  (UserInterface|Viewport|AddtoViewport _returnvalue_2 0))

(event EventTick
  (params (DeltaSeconds :type Float%20%28single-precision%29))
  (bind _returnvalue (Game|GetPlayerController 0))
  (bind _array (Utilities|Array|MakeArray "ObjectTypeQuery2"))
  (bind (_hitresult _returnvalue_2) (Class|PlayerController|GetHitResultUnderCursorforObjects _returnvalue _array true))
  ;[0 0.7604 0.5839] Select robot
  (if _returnvalue_2
    (bind _asbp_jackal_robot (Utilities|Casting|CastToBP_JackalRobot (.HitActor (Collision|BreakHitResult _hitresult)))
      (:then
        (CallFunction|UpdateHoveredJackal _asbp_jackal_robot))
      (:CastFailed
        (CallFunction|UpdateHoveredJackal :!label _label)))
    (else
      (goto _label))))

(event Input|MouseEvents|MouseX
  (params (AxisValue :type Float%20%28single-precision%29))
  ;[0 0.7604 0.5839] Movement
  (Pawn|Input|AddControllerYawInput AxisValue))

(event Input|MouseEvents|MouseY
  (params (AxisValue :type Float%20%28single-precision%29))
  ;[0 0.7604 0.5839] Movement
  (Pawn|Input|AddControllerPitchInput (* AxisValue -1.0)))

(event Input|KeyboardEvents|LeftCtrl
  (params (Key :type Key%20Structure :default "None"))
  ;[0 0.7604 0.5839] Select robot
  (:Pressed
    (bind _isa (Utilities|FlowControl|FlipFlop)
      (:A
        _)
      (:B
        _))
    (Variables|/Script/Engine.PlayerController|SetbShowMouseCursor (Game|GetPlayerController 0) _isa)))

(event Input|MouseEvents|LeftMouseButton
  (params (Key :type Key%20Structure :default "None"))
  (bind _hoveredjackal (Variables|Default|GethoveredJackal))
  ;[0 0.7604 0.5839] Select robot
  (:Pressed
    (Utilities|IsValid _hoveredjackal
      (:Is%20Valid
        (Default|UpdateCurrentJackal (Variables|Default|GetjackalControlUI) _hoveredjackal)))))

(event Input|KeyboardEvents|Escape
  (params (Key :type Key%20Structure :default "None"))
  ;[0 0.7604 0.5839] Movement
  (:Pressed
    (Game|QuitGame 0 "Quit" false)))

(fn ConstructionScript)