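; Workstation prop where JackalRobots work together on a timed task while its Reward is positive.
; Overlapping robots are tracked, and their blackboards receive in-station state, task duration and a wait timestamp, refreshed for all on each new arrival.
; Tick updates billboard text and gear or checkmark sprites, counting down only while enough robots are working.
; At zero it calls FinishPropTask and clears the robots' in-station flags.
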(event Collision|EventActorBeginOverlap
  (params (OtherActor :type Actor%20Object%20Reference))
  (bind _asjackal_robot (Utilities|Casting|CastToJackalRobot OtherActor))
  (Utilities|Array|Add (Variables|Default|GetOverlappedJackals) _asjackal_robot)
  (if (> (Variables|Default|GetReward) 0.0)
    (|InitializeWorker _asjackal_robot)))

(event EventTick
  (params (DeltaSeconds :type Float%20%28single-precision%29))
  (bind _activeworkers (CallFunction|GetActiveWorokers))
  (if (> (Variables|Default|GetReward) 0.0)
    (Default|SetText (Variables|Default|GetBillboardTextRender) (Utilities|String|Append (Utilities|String|ToString(Integer) (Utilities|Array|Length (Variables|Default|GetOverlappedJackals))) " 
" (Utilities|String|ToString(Integer) _activeworkers) "/" (Utilities|String|ToString(Integer) (Variables|Default|GetRequiredWorkers))))
    (if (>= _activeworkers (Variables|Default|GetRequiredWorkers))
      (bind _output_get (Variables|Default|SetTaskRemainingTime (- (Variables|Default|GetTaskRemainingTime) DeltaSeconds)))
      (if (<= _output_get 0.0)
        (Rendering|Components|Sprite|SetSprite (Variables|Default|GetBillboard) "/Game/Core/StatusIcons/check-mark.check-mark")
        (Class|JackalInteractiveProp|FinishPropTask)
        (for _array_element (Variables|Default|GetOverlappedJackals)
          (AI|Components|Blackboard|SetValueasBool (AI|GetBlackboard _array_element) (Utilities|Name|MakeLiteralName "InWorkStation") false))
        (else
          (Rendering|Components|Sprite|SetSprite (Variables|Default|GetBillboard) "/Game/Core/StatusIcons/gears-in-progress.gears-in-progress")))
      (else
        (Rendering|Components|Sprite|SetSprite (Variables|Default|GetBillboard) "/Game/Core/StatusIcons/gear-alone.gear-alone")))))

(event Collision|EventActorEndOverlap
  (params (OtherActor :type Actor%20Object%20Reference))
  (bind _asjackal_robot (Utilities|Casting|CastToJackalRobot OtherActor))
  (Utilities|Array|RemoveItem (Variables|Default|GetOverlappedJackals) _asjackal_robot)
  (AI|Components|Blackboard|SetValueasBool (AI|GetBlackboard _asjackal_robot) (Utilities|Name|MakeLiteralName "InWorkStation") false))

(event EventBeginPlay
  (Variables|Default|SetTaskRemainingTime (Variables|Default|GetTaskTime))
  (bind _asbp_billboard_text_render (Utilities|Casting|CastToBP_BillboardTextRender (Variables|/Script/Engine.ChildActorComponent|GetChildActor (Variables|Default|GetBP_BillboardTextRender))))
  (Variables|Default|SetBillboardTextRender _asbp_billboard_text_render))

(fn ConstructionScript)

(fn GetActiveWorokers
  (for _array_element (Variables|Default|GetOverlappedJackals)
    (if (and (Utilities|IsValid _array_element) (Variables|/Script/Beryl.JackalRobot|GetbIsWorking _array_element))
      (Math|Integer|IncrementInt (LocalVariables|GetWorkingJackals))))
  (return (LocalVariables|GetWorkingJackals)))