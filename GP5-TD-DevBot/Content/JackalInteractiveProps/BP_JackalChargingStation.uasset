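; BP_JackalChargingStation is a prop that recharges Jackal robots while they overlap it.
; Overlap events maintain a list of robots inside and set each one's InChargingStation blackboard bool for its AI.
; Every Tick it recharges each listed robot's battery by delta time scaled by a charging speed multiplier.
; A billboard text child actor, cached on BeginPlay, displays the current robot count.
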(event EventBeginPlay
  (bind _asbp_billboard_text_render (Utilities|Casting|CastToBP_BillboardTextRender (Variables|/Script/Engine.ChildActorComponent|GetChildActor (Variables|Default|GetBP_BillboardTextRender))))
  (Variables|Default|SetBillboardTextRender _asbp_billboard_text_render))

(event Collision|EventActorBeginOverlap
  (params (OtherActor :type Actor%20Object%20Reference))
  (bind _asbp_jackal_robot (Utilities|Casting|CastToBP_JackalRobot OtherActor))
  (if (not (Utilities|Array|ContainsItem (Variables|Default|GetOverlappingJackals) _asbp_jackal_robot))
    (Utilities|Array|Add (Variables|Default|GetOverlappingJackals) _asbp_jackal_robot)
    (AI|Components|Blackboard|SetValueasBool (AI|GetBlackboard _asbp_jackal_robot) (Utilities|Name|MakeLiteralName "InChargingStation") true)))

(event Collision|EventActorEndOverlap
  (params (OtherActor :type Actor%20Object%20Reference))
  (bind _asbp_jackal_robot (Utilities|Casting|CastToBP_JackalRobot OtherActor))
  (Utilities|Array|RemoveItem (Variables|Default|GetOverlappingJackals) _asbp_jackal_robot)
  (AI|Components|Blackboard|SetValueasBool (AI|GetBlackboard _asbp_jackal_robot) (Utilities|Name|MakeLiteralName "InChargingStation") false))

(event EventTick
  (params (DeltaSeconds :type Float%20%28single-precision%29))
  (Default|SetText (Variables|Default|GetBillboardTextRender) (Utilities|String|ToString(Integer) (Utilities|Array|Length (Variables|Default|GetOverlappingJackals))))
  (for _array_element (Variables|Default|GetOverlappingJackals)
    (Class|JackalRobot|RechargeBattery _array_element (* DeltaSeconds (Variables|Default|GetChargingSpeedMultiplier)))))

(fn ConstructionScript)