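; BP_DedicatedJackalTarget is an interactive prop that serves as a task target for one dedicated Jackal robot.
; On BeginPlay it picks a random Jackal if none is valid, then shows the robot's ID on a child-actor billboard.
; Overlap by the dedicated robot with positive Reward finishes the task.
; Otherwise, any overlapping Jackal records the prop's ID in its visited-target list.
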(event Custom|UpdateText
  (bind _asbp_billboard_text_render (Utilities|Casting|CastToBP_BillboardTextRender (Variables|/Script/Engine.ChildActorComponent|GetChildActor (Variables|Default|GetBP_BillboardTextRender))))
  (bind _dedicatedrobot (Variables|Default|GetDedicatedRobot)
    (:then
      (Utilities|FlowControl|DelayUntilNextTick)
      (Default|SetText _asbp_billboard_text_render (Utilities|String|Append "Jackal" (Utilities|String|ToString(Integer) (Class|JackalRobot|GetJackalId _dedicatedrobot)))))
    (:else
      (Default|SetText _asbp_billboard_text_render "[No valid Jackal]"))))

(event Collision|EventActorBeginOverlap
  (params (OtherActor :type Actor%20Object%20Reference))
  (if (and (== OtherActor (Variables|Default|GetDedicatedRobot)) (> (Variables|Default|GetReward) 0.0))
    (CallFunction|FinishTask)
    (else
      (bind _asbp_jackal_robot (Utilities|Casting|CastToBP_JackalRobot OtherActor))
      (Utilities|Array|AddUnique (Variables|/Game/JackalRobot/Pawn/BP_JackalRobot.BP_JackalRobot_C|GetDedicatedTargetVisited _asbp_jackal_robot) (Class|JackalInteractiveProp|GetPropId)))))

(event EventBeginPlay
  (Variables|Default|GetDedicatedRobot
    (:then
      (CallFunction|UpdateText))
    (:else
      (CallFunction|AssigntoRandomJackal))))

(fn ConstructionScript
  (|CallParentFunction))

(fn AssigntoRandomJackal
  (bind _outactors (Actor|GetAllActorsOfClass "/Script/Beryl.JackalRobot"))
  (Variables|Default|SetDedicatedRobot (.OutItem (Utilities|Array|Random _outactors)))
  (CallFunction|UpdateText))